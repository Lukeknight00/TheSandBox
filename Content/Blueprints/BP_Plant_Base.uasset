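; BP_Plant_Base is a procedural plant segment that spends energy to grow and buds new segments into a chain.
; Each Tick, Grow scales the cylinder while energy covers the rising cost, losing health otherwise, until it reaches maximum size.
; It then spawns one half-scale child plant, offset upward by the cylinder's local bounds, and on later ticks overwrites that child's energy with its own.
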(event `self.ReceiveBeginPlay`)

(event `self.ReceiveTick`
  (params (DeltaSeconds :type "Float (single-precision)"))
  (if (`self.Growable`)
    (bind _remainingenergy (`self.Grow` (`self.Energy`)))
    (set `self.Energy` _remainingenergy)
    (elif (`self.budded`)
      (`self.TransferEnergy` self (`self.Energy`) (stale _output_get))
      (else
        (bind _returnvalue (`self.Bud`))
        (bind _output_get (set `self.ChildPlant` _returnvalue))
        (set `self.budded` true)))))

(fn `Bud`
  (returns (ReturnValue :type "/Game/Blueprints/BP_Plant_Base Object Reference"))
  (bind _cylinder (`self.Cylinder`))
  (bind (_returnvalue_location _returnvalue_rotation) (`KismetMathLibrary.BreakTransform` (`SceneComponent.K2_GetComponentToWorld` _cylinder)))
  (bind _returnvalue (`|SpawnActorFromClass` "BP_Plant_Base_C" (`KismetMathLibrary.MakeTransform` (+ _returnvalue_location (`KismetMathLibrary.MakeVector` 0.0 0.0 (.z (`.Max` (`StaticMeshComponent.GetLocalBounds` _cylinder))))) _returnvalue_rotation (0.5 0.5 0.5)) "AlwaysSpawn" "OverrideRootScale" null (`self.Energy`) null))
  (return _returnvalue))

(fn `Grow`
  (params (EnergySupplied :type "Float (double-precision)"))
  (returns (RemainingEnergy :type "Float (double-precision)"))
  (locals (RemEnergy :type "Float (double-precision)" :default 0.0))
  (bind _cylinder (`self.Cylinder`))
  (bind (_returnvalue_x _returnvalue_y _returnvalue_z) (`KismetMathLibrary.BreakVector` (`SceneComponent.K2_GetComponentScale` (`self.Cylinder`))))
  (bind _output_get (set `self.CurrentSize` (`KismetMathLibrary.Sqrt` (+ (`KismetMathLibrary.Square` _returnvalue_x) (`KismetMathLibrary.Square` _returnvalue_y) (`KismetMathLibrary.Square` _returnvalue_z)))))
  (`KismetSystemLibrary.PrintString` (`KismetStringLibrary.Conv_DoubleToString` _output_get) true true (struct :`G` 0.66 :`B` 1.0 :`A` 1.0) 0.05)
  (if (> (`self.MaxSize`) (`self.CurrentSize`))
    (if (> EnergySupplied (`self.EnergyCost`))
      (`SceneComponent.SetRelativeScale3D` _cylinder (* (`SceneComponent.RelativeScale3D` _cylinder) (`self.GrowthRate`)))
      (bind _output_get_2 (set `local.RemEnergy` (- EnergySupplied (`self.EnergyCost`))))
      (set `self.EnergyCost` (* (`self.EnergyCost`) (`self.GrowthRate`)))
      (return _output_get_2)
      (else
        (set `self.Health` (- (`self.Health`) 1.0))))
    (else
      (set `self.Growable` false)))
  (return EnergySupplied))

(fn `Set Initial Energy`
  (params (inputEnergy :type "Float (double-precision)"))
  (set `self.Energy` inputEnergy))

(fn `TransferEnergy`
  (params (Energy :type "Float (double-precision)") (AdjacentPlant :type "Actor Object Reference"))
  (bind _asbp_plant_base (cast `/Game/Blueprints/BP_Plant_Base` AdjacentPlant))
  (set `/Game/Blueprints/BP_Plant_Base.Energy` Energy _asbp_plant_base)
  (set `self.Energy` 0.0))

(fn `UserConstructionScript`)
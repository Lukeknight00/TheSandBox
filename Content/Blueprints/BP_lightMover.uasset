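; BP_lightMover is an actor that spawns a BP_LightSource and orbits it around the world origin.
; On BeginPlay it spawns the light at a height equal to the rotation radius, passing photon energy, distance and power, and stores its sphere's position.
; Each Tick rotates that stored vector around a configurable axis by a fixed, frame-rate-dependent angle and moves the light there.
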(event `self.ReceiveBeginPlay`
  (bind _returnvalue (`|SpawnActorFromClass` "/Game/Blueprints/BP_LightSource.BP_LightSource_C" (`KismetMathLibrary.MakeTransform` (`KismetMathLibrary.MakeVector` 0.0 0.0 (`self.Light Rotation Radius`))) "Undefined" "OverrideRootScale" null (`self.Photon Energy`) (`self.Light Distance`) (`self.Light Power`) null))
  (bind _output_get (set `self.LightSource` _returnvalue))
  (set `self.CurrentPosition` (`SceneComponent.K2_GetComponentLocation` (`/Game/Blueprints/BP_LightSource.Sphere` _output_get))))

(event `self.ReceiveTick`
  (params (DeltaSeconds :type "Float (single-precision)"))
  (bind _returnvalue (`KismetMathLibrary.RotateAngleAxis` (`self.CurrentPosition`) (`self.Roatation Speed`) (`self.AxisOfRotation`)))
  (`self.K2_SetActorTransform` (`self.LightSource`) (`KismetMathLibrary.Conv_VectorToTransform` _returnvalue) false false)
  (set `self.CurrentPosition` _returnvalue))

(fn `UserConstructionScript`)
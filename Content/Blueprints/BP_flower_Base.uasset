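; Base flower actor that seeds further plants as soon as it begins play, then destroys itself after its LifeSpan delay.
; Seed spawns a BP_plantspawner at the Sphere's XY and a fixed Z, passing seed count and a height range built from Height and HeightVariance.
; The spawner's area starts at the flower's position and extends by a random fraction of DistributionRange in X and Y, so it is not centered on the flower.
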(event `self.ReceiveBeginPlay`
  (`self.Seed`)
  (`KismetSystemLibrary.Delay` (`self.LifeSpan`))
  (`self.K2_DestroyActor`))

(fn `Seed`
  (bind _heightvariance (`self.HeightVariance`))
  (bind _height (`self.Height`))
  (bind (_returnvalue_x _returnvalue_y) (`KismetMathLibrary.BreakVector` (`SceneComponent.K2_GetComponentLocation` (`self.Sphere`))))
  (`|SpawnActorFromClass` "/Game/Blueprints/BP_plantspawner.BP_plantspawner_C" (`KismetMathLibrary.MakeTransform` (`KismetMathLibrary.MakeVector` _returnvalue_x _returnvalue_y 20.0)) "AdjustIfPossibleButAlwaysSpawn" "OverrideRootScale" null (`self.Seeds`) (+ _returnvalue_x (* (`self.DistributionRange`) (`KismetMathLibrary.RandomFloat`))) (+ _returnvalue_y (* (`self.DistributionRange`) (`KismetMathLibrary.RandomFloat`))) _returnvalue_x _returnvalue_y (- _height _heightvariance) (+ _height _heightvariance) null)
  (return))

(fn `UserConstructionScript`)
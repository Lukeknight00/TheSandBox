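; BP_plantspawner is a one-shot spawner that scatters BP_Plant_Base actors over a rectangular area when play begins.
; BeginPlay loops over NumberOfSeeds, spawning each plant at random world X/Y within the configured bounds and a fixed Z, adjusting for collisions but always spawning.
; Each plant receives a random MaxHeight from the spawner's height range.
; The spawner destroys itself once the loop finishes.
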(event `self.ReceiveBeginPlay`
  (for _ (range (+ (`self.NumberOfSeeds`) 1))
    (`|SpawnActorFromClass` "/Game/Blueprints/BP_Plant_Base.BP_Plant_Base_C" (`KismetMathLibrary.MakeTransform` (`KismetMathLibrary.MakeVector` (`KismetMathLibrary.RandomFloatInRange` (`self.xLowerBound`) (`self.xUpperBound`)) (`KismetMathLibrary.RandomFloatInRange` (`self.yLowerBound`) (`self.yUpperBound`)) 10.0)) "AdjustIfPossibleButAlwaysSpawn" "OverrideRootScale" null 10000.0 (`KismetMathLibrary.RandomFloatInRange` (`self.MinHight`) (`self.MaxHeight`)) null))
  (`self.K2_DestroyActor`))

(fn `UserConstructionScript`)
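; BP_LightSource is a light actor that feeds energy to plants by simulating photons with random raycasts.
; Each tick it calls EmitEnergy once per whole unit of LightPower.
; Each call traces the Visibility channel from the Light in a random direction up to LightDistance, adding PhotonEnergy to the Energy of any BP_Plant_Base it hits first.
; Energy delivered scales with tick rate, since delta time is not used.
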(event `self.ReceiveTick`
  (params (DeltaSeconds :type "Float (single-precision)"))
  (for _ (range (+ (`KismetMathLibrary.FTrunc` (`self.LightPower`)) 1))
    (`self.EmitEnergy`)))

(fn `EmitEnergy`
  (bind _returnvalue (`SceneComponent.K2_GetComponentLocation` (`self.Light`)))
  (bind _outhit (`KismetSystemLibrary.LineTraceSingle` _returnvalue (+ (* (`KismetMathLibrary.RandomUnitVector`) (`self.LightDistance`)) _returnvalue) "TraceTypeQuery1"))
  (bind _asbp_plant_base (cast `/Game/Blueprints/BP_Plant_Base` (`.HitActor` (`GameplayStatics.BreakHitResult` _outhit))))
  (set `/Game/Blueprints/BP_Plant_Base.Energy` (+ (`/Game/Blueprints/BP_Plant_Base.Energy` _asbp_plant_base) (`self.PhotonEnergy`)) _asbp_plant_base))

(fn `UserConstructionScript`)